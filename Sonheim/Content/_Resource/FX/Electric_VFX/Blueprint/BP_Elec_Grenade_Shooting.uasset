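; Electric VFX Blueprint that repeatedly shoots projectile actors, apparently grenades going by the asset name.
; One second after BeginPlay it spawns the projectile class at a small random offset from its location, scaled down and rotated to match its Arrow component.
; The NextArrow event then re-triggers itself after a random delay of a few seconds, looping the fire with no stop condition.
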(event Custom|NextArrow
  (bind _returnvalue (Math|Random|RandomFloatinRange -25.0 25.0))
  (Game|SpawnActorfromClass (Variables|Default|GetProjectileBP) (Math|Transform|MakeTransform (+ (Transformation|GetActorLocation) (Math|Vector|MakeVector _returnvalue _returnvalue _returnvalue)) (.rotation (Transformation|GetWorldTransform (Variables|Default|GetArrow))) "0.100000,0.100000,0.100000") "AlwaysSpawn" "SelectDefaultAtRuntime" 0 0)
  (Utilities|FlowControl|Delay (Math|Random|RandomFloatinRange 3.0 4.0))
  (CallFunction|NextArrow))

(event EventBeginPlay
  (bind _returnvalue (Math|Random|RandomFloatinRange -25.0 25.0))
  (Utilities|FlowControl|Delay 1.0)
  (Game|SpawnActorfromClass (Variables|Default|GetProjectileBP) (Math|Transform|MakeTransform (+ (Transformation|GetActorLocation) (Math|Vector|MakeVector _returnvalue _returnvalue _returnvalue)) (.rotation (Transformation|GetWorldTransform (Variables|Default|GetArrow))) "0.100000,0.100000,0.100000") "AlwaysSpawn" "SelectDefaultAtRuntime" 0 0)
  (Utilities|FlowControl|Delay (Math|Random|RandomFloatinRange 3.0 4.0))
  (CallFunction|NextArrow))

(fn ConstructionScript)