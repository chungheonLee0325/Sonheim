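; BP_Projectile_01 is a fire projectile effect actor that plays Niagara shot, trail and hit effects.
; BeginPlay spawns the fire shot system just in front of the actor.
; A SphereCollider hit spawns the fire hit system, alongside a spawn call with no template set, and removes the first ribbon trail.
; The second trail lingers briefly through a delay before it and the actor are destroyed.
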(event OnComponentHit(SphereCollider)
  (params (HitComponent :type Primitive%20Component%20Object%20Reference) (OtherActor :type Actor%20Object%20Reference) (OtherComp :type Primitive%20Component%20Object%20Reference) (NormalImpulse :type Vector :default "0, 0, 0") (Hit :type Hit%20Result%20Structure%20%28by%20ref%29))
  (bind _sphere_collider (Variables|Default|GetSphere%20Collider))
  (bind _sphere_collider_2 (Variables|Default|GetSphere%20Collider))
  (Niagara|SpawnSystematLocation 0 (Transformation|GetWorldLocation _sphere_collider) (Transformation|GetWorldRotation _sphere_collider))
  (Components|DestroyComponent (Variables|Default|GetNS_RibbonTrail_01))
  (Niagara|SpawnSystematLocation "/Game/_Resource/FX/Effect/NiagaraSystems/FireBullet/NS_Fire_Hit_01.NS_Fire_Hit_01" (Transformation|GetWorldLocation _sphere_collider_2) (Transformation|GetWorldRotation _sphere_collider_2))
  (Utilities|FlowControl|Delay 0.6)
  (Components|DestroyComponent (Variables|Default|GetNS_RibbonTrail_02))
  (Actor|DestroyActor))

(event EventBeginPlay
  (bind _returnvalue (Transformation|GetActorTransform))
  (Niagara|SpawnSystematLocation "/Game/_Resource/FX/Effect/NiagaraSystems/FireBullet/NS_Fire_Shot_01.NS_Fire_Shot_01" (Math|Transform|TransformLocation _returnvalue "50.000000,0.000000,0.000000") (Math|Transform|TransformRotation _returnvalue "0, 0, 0")))

(fn ConstructionScript)