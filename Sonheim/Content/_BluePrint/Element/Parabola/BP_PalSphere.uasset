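; Pal Sphere actor, a monster-capture ball that presents the capture sequence and destroys itself ten seconds after spawning.
; Capture reveal events set Hit or Fail flags on its ABP_PalSphere animation blueprint and spawn Niagara effects for success or failure.
; Each filled segment spawns a shot effect aligned to the sphere with inverted pitch.
; The overlap handler only calls an empty TEST event; older monster-activation and physics-bounce logic remains disconnected.
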(event Custom|TEST
  (params (Caster :type Area%20Object%20Object%20Reference) (Target :type Actor%20Object%20Reference)))

(event EventBeginPlay
  (|CallParentFunction)
  (Utilities|FlowControl|Delay 1e+01)
  (Actor|DestroyActor))

(event Collision|EventActorBeginOverlap
  (params (OtherActor :type Actor%20Object%20Reference)))

(event EventTick
  (params (DeltaSeconds :type Float%20%28single-precision%29)))

(event EventHandleBeginOverlap
  (params (Caster :type Area%20Object%20Object%20Reference) (Target :type Actor%20Object%20Reference))
  (CallFunction|TEST Caster Target))

(event EventOnCaptureRevealStart
  (bind _asabp_pal_sphere (Utilities|Casting|CastToABP_PalSphere (Components|SkeletalMesh|GetAnimInstance (Variables|Default|GetSkeletalMesh))))
  (Variables|/Game/_BluePrint/Element/Parabola/ABP_PalSphere.ABP_PalSphere_C|SetbHit _asabp_pal_sphere true))

(event EventOnCaptureRevealEnd
  (params (bSuccess :type Boolean))
  (if bSuccess
    (Utilities|FlowControl|Delay 0.5)
    (Niagara|SpawnSystematLocation "/Game/_Resource/FX/Effect/NiagaraSystems/MagicBullet/NS_BlueBullet_Hit_01.NS_BlueBullet_Hit_01" (Transformation|GetActorLocation) (Transformation|GetActorRotation))
    (else
      (bind _asabp_pal_sphere (Utilities|Casting|CastToABP_PalSphere (Components|SkeletalMesh|GetAnimInstance (Variables|Default|GetSkeletalMesh))))
      (Variables|/Game/_BluePrint/Element/Parabola/ABP_PalSphere.ABP_PalSphere_C|SetbFail _asabp_pal_sphere true)
      (Niagara|SpawnSystematLocation "/Game/_Resource/FX/Effect/NiagaraSystems/DarkBullet/Fail.Fail" (Transformation|GetActorLocation) (Transformation|GetActorRotation)))))

(event EventOnSegmentFilled
  (params (SegmentIndex :type Integer))
  (bind _returnvalue (Transformation|GetActorRotation))
  (Niagara|SpawnSystematLocation "/Game/_Resource/FX/Effect/NiagaraSystems/MagicBullet/NS_BlueShot_01.NS_BlueShot_01" (Transformation|GetActorLocation) (Math|Rotator|MakeRotator (.roll _returnvalue) (* (.pitch _returnvalue) -1.0) (.yaw _returnvalue)) "0.800000,0.800000,0.800000"))

(fn ConstructionScript)