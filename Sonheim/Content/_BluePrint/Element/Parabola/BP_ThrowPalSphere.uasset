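; BP_ThrowPalSphere is a thrown capture sphere that lets a Sonheim player claim a monster as a partner.
; Its overlap handler casts the target to BaseMonster and the caster to SonheimPlayer, then rejects monsters that already have a PartnerOwner.
; Otherwise a random integer roll decides whether the player becomes the partner owner; the roll succeeds 70% of the time, despite a 60% comment.
; Rejections and failed rolls only print debug strings.
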(event EventBeginPlay)

(event Collision|EventActorBeginOverlap
  (params (OtherActor :type Actor%20Object%20Reference)))

(event EventTick
  (params (DeltaSeconds :type Float%20%28single-precision%29)))

(event EventHandleBeginOverlap
  (params (Caster :type Area%20Object%20Object%20Reference) (Target :type Actor%20Object%20Reference))
  (bind _asbase_monster (Utilities|Casting|CastToBaseMonster Target))
  (bind _assonheim_player (Utilities|Casting|CastToSonheimPlayer Caster))
  (if (Utilities|IsValid (Variables|/Script/Sonheim.BaseMonster|GetPartnerOwner _asbase_monster))
    (Development|PrintString "have a owner already")
    (elif (>= (Math|Random|RandomIntegerinRange 1 10) 4)
      (Class|BaseMonster|SetPartnerOwner _asbase_monster _assonheim_player)
      (else
        (Development|PrintString "확률 실패!")))))

(fn ConstructionScript)