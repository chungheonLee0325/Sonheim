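; Player Blueprint that layers test hotkeys and a stair repair relay over its parent class.
; Number, symbol, letter and numpad keys grant fixed items through the player state's inventory component or Reward calls, and add experience through the level component.
; RestoreStair forwards to RepairStair, which passes item ID and amount to the BP_Stair found in the level.
; Tick only calls the parent, and leftover debug and partner-spawning nodes are disconnected.
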(event Custom|RepairStair
  (params (ItemID :type Integer) (Value :type Integer))
  (bind _returnvalue (Actor|GetActorOfClass "/Game/_BluePrint/GameObject/BP_Stair.BP_Stair_C"))
  (Default|RepairStair _returnvalue ItemID Value))

(event EventBeginPlay)

(event Collision|EventActorBeginOverlap
  (params (OtherActor :type Actor%20Object%20Reference)))

(event EventTick
  (params (DeltaSeconds :type Float%20%28single-precision%29))
  (|CallParentFunction DeltaSeconds))

(event EventRestoreStair
  (params (ItemID :type Integer) (ItemCount :type Integer))
  (CallFunction|RepairStair ItemID ItemCount))

(event Input|KeyboardEvents|7
  (params (Key :type Key%20Structure :default "None"))
  ;[0.15 0 0.06539 0.5] TestZone
  (:Pressed
    (Class|InventoryComponent|AddItem (Variables|/Script/Sonheim.SonheimPlayerState|Getm_InventoryComponent (Class|SonheimPlayer|GetSPlayerState)) 100 1 true)))

(event Input|KeyboardEvents|8
  (params (Key :type Key%20Structure :default "None"))
  ;[0.15 0 0.06539 0.5] TestZone
  (:Pressed
    (Class|InventoryComponent|AddItem (Variables|/Script/Sonheim.SonheimPlayerState|Getm_InventoryComponent (Class|SonheimPlayer|GetSPlayerState)) 101 1 true)))

(event Input|KeyboardEvents|M
  (params (Key :type Key%20Structure :default "None")))

(event Input|KeyboardEvents|Period
  (params (Key :type Key%20Structure :default "None")))

(event Input|KeyboardEvents|M
  (params (Key :type Key%20Structure :default "None"))
  (:Pressed
    (Class|SonheimPlayer|Reward 1 4)))

(event Input|KeyboardEvents|Period
  (params (Key :type Key%20Structure :default "None"))
  (:Pressed
    (Class|SonheimPlayer|Reward 10 4)))

(event Input|KeyboardEvents|Comma
  (params (Key :type Key%20Structure :default "None"))
  (:Pressed
    (Class|SonheimPlayer|Reward 5 4)))

(event Input|KeyboardEvents|NumPadFour
  (params (Key :type Key%20Structure :default "None"))
  (:Pressed
    (Class|SonheimPlayer|Reward 500 5)))

(event Input|KeyboardEvents|Slash
  (params (Key :type Key%20Structure :default "None"))
  (:Pressed
    (Class|SonheimPlayer|Reward 15 4)))

(event Input|KeyboardEvents|NumPadFive
  (params (Key :type Key%20Structure :default "None"))
  (:Pressed
    (Class|SonheimPlayer|Reward 1000 12)))

(event Input|KeyboardEvents|9
  (params (Key :type Key%20Structure :default "None"))
  ;[0.15 0 0.06539 0.5] TestZone
  (:Pressed
    (Class|InventoryComponent|AddItem (Variables|/Script/Sonheim.SonheimPlayerState|Getm_InventoryComponent (Class|SonheimPlayer|GetSPlayerState)) 200 1 true)))

(event Input|KeyboardEvents|0
  (params (Key :type Key%20Structure :default "None"))
  ;[0.15 0 0.06539 0.5] TestZone
  (:Pressed
    (Class|InventoryComponent|AddItem (Variables|/Script/Sonheim.SonheimPlayerState|Getm_InventoryComponent (Class|SonheimPlayer|GetSPlayerState)) 110 1 true)))

(event Input|KeyboardEvents|Hyphen
  (params (Key :type Key%20Structure :default "None"))
  ;[0.15 0 0.06539 0.5] TestZone
  (:Pressed
    (Class|InventoryComponent|AddItem (Variables|/Script/Sonheim.SonheimPlayerState|Getm_InventoryComponent (Class|SonheimPlayer|GetSPlayerState)) 120 1 true)))

(event Input|KeyboardEvents|O
  (params (Key :type Key%20Structure :default "None"))
  (:Pressed
    (Class|LevelComponent|AddExp (Variables|Default|Getm_LevelComponent) 3)))

(event Input|KeyboardEvents|Equals
  (params (Key :type Key%20Structure :default "None"))
  ;[0.15 0 0.06539 0.5] TestZone
  (:Pressed
    (Class|InventoryComponent|AddItem (Variables|/Script/Sonheim.SonheimPlayerState|Getm_InventoryComponent (Class|SonheimPlayer|GetSPlayerState)) 150 1 true)))

(event Input|KeyboardEvents|U
  (params (Key :type Key%20Structure :default "None"))
  (:Pressed
    (Class|LevelComponent|AddExp (Variables|Default|Getm_LevelComponent) 999)))

(event Input|KeyboardEvents|Slash
  (params (Key :type Key%20Structure :default "None")))

(event Input|KeyboardEvents|Comma
  (params (Key :type Key%20Structure :default "None")))

(fn ConstructionScript)