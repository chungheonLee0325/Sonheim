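; BP_BaseMonster is a monster Blueprint that automatically attacks the player shortly after play begins.
; BeginPlay sets the capsule to the Monster collision profile and hard-codes its area object ID.
; After a short delay it takes the first player pawn as aggro target and casts a skill, looked up by ID, on it.
; Two disconnected chains that would cast other skills on the monster itself never run.
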(event EventBeginPlay
  (Collision|SetCollisionProfileName (Variables|Default|GetCapsuleComponent) "Monster" true :!class /Script/Engine.PrimitiveComponent)
  (Variables|Default|Setm_AreaObjectID 109)
  (Utilities|FlowControl|Delay 3.0)
  (bind _asbp_player (Utilities|Casting|CastToBP_Player (Game|Player|GetPlayerPawn 0)))
  (Class|BaseMonster|SetAggroTarget _asbp_player)
  (bind _returnvalue (Class|AreaObject|GetSkillbyID 1090))
  (Class|AreaObject|CastSkill _returnvalue _asbp_player))

(fn ConstructionScript)