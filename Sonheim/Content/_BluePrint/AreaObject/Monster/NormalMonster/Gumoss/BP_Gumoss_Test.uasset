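; BP_Gumoss_Test is a test variant of the Gumoss normal monster that becomes the player's partner.
; Half a second after BeginPlay, it casts the first player pawn to SonheimPlayer and sets it as its partner owner.
; Disconnected leftover nodes would cast skills by ID on itself, one after a delay, but never run.
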(event EventBeginPlay
  (Utilities|FlowControl|Delay 0.5)
  (bind _assonheim_player (Utilities|Casting|CastToSonheimPlayer (Game|Player|GetPlayerPawn 0)))
  (Class|BaseMonster|SetPartnerOwner _assonheim_player))

(event Collision|EventActorBeginOverlap
  (params (OtherActor :type Actor%20Object%20Reference)))

(event EventTick
  (params (DeltaSeconds :type Float%20%28single-precision%29)))

(fn ConstructionScript)