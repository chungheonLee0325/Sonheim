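; BP_Stair is a repairable staircase that players rebuild by contributing wood, stone, ore and Paldium.
; RepairStair adds capped amounts per item ID, updates the WB_Stair progress bars shown from BeginPlay, and sets a flag as each material fills.
; Tick watches the four flags and calls FlagControl once, switching the MPC_Color parameter, enabling collision on the floor and stair meshes, spawning effects and removing the widget.
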(event OnComponentBeginOverlap(Box)
  (params (OverlappedComponent :type Primitive%20Component%20Object%20Reference) (OtherActor :type Actor%20Object%20Reference) (OtherComp :type Primitive%20Component%20Object%20Reference) (OtherBodyIndex :type Integer) (bFromSweep :type Boolean) (SweepResult :type Hit%20Result%20Structure%20%28by%20ref%29))
  (if (not (Variables|Default|GetIsFlag))
    (Utilities|Casting|CastToSonheimPlayer OtherActor)))

(event OnComponentEndOverlap(Box)
  (params (OverlappedComponent :type Primitive%20Component%20Object%20Reference) (OtherActor :type Actor%20Object%20Reference) (OtherComp :type Primitive%20Component%20Object%20Reference) (OtherBodyIndex :type Integer))
  (if (not (Variables|Default|GetIsFlag))
    (Utilities|Casting|CastToSonheimPlayer OtherActor)))

(event Custom|FlagControl
  (params (Flag :type Boolean))
  (bind _scene (Variables|Default|GetScene))
  (bind _returnvalue (Transformation|GetWorldLocation _scene))
  (if Flag
    (Rendering|Material|SetScalarParameterValue "/Game/_Resource/SurvivalGameKitV2/Materials/BuildParts/MPC_Color.MPC_Color" "Flag" 0.0 :!class /Script/Engine.KismetMaterialLibrary)
    (for _array_element (Variables|Default|GetMeshArray)
      (Collision|SetCollisionEnabled _array_element "QueryAndPhysics")
      (Effects|SpawnEmitteratLocation "/Game/_Resource/FX/VFX_Toolkit_V1/ParticleSystems/356Days/Par_ToonKaboom_02.Par_ToonKaboom_02" (Math|Vector|MakeVector (.x _returnvalue) (.y _returnvalue) (+ (.z _returnvalue) 1.8e+02)) "0, 0, 0" "2.500000,2.500000,2.500000")
      (Widget|RemovefromParent (Variables|Default|GetWB_Stair)))
    (else
      (Rendering|Material|SetScalarParameterValue "/Game/_Resource/SurvivalGameKitV2/Materials/BuildParts/MPC_Color.MPC_Color" "Flag" 1.0 :!class /Script/Engine.KismetMaterialLibrary)
      (for _array_element_2 (Variables|Default|GetMeshArray)
        (Collision|SetCollisionEnabled _array_element_2 "NoCollision")))))

(event Custom|RepairStair
  (params (ItemID :type Integer) (Value :type Integer))
  (bind _wb_stair (Variables|Default|GetWB_Stair))
  (if (== ItemID 1)
    (bind _output_get (Variables|Default|SetWoodCurrent (Math|Integer|Min(Integer) (+ (stale _output_get) Value) 20)))
    (Progress|SetPercent (Variables|/Game/_BluePrint/Widget/WB_Stair.WB_Stair_C|GetWoodProgressBar _wb_stair) (/ (Math|Conversions|ToFloat(Integer) _output_get) 2e+01))
    (bind _output_get_2 (Variables|Default|SetwoodFlag (== (/ (Math|Conversions|ToFloat(Integer) _output_get) 2e+01) 1.0)))
    (elif (== ItemID 5)
      (bind _output_get_3 (Variables|Default|SetStoneCurrent (Math|Integer|Min(Integer) (+ (stale _output_get_3) Value) 20)))
      (Progress|SetPercent (Variables|/Game/_BluePrint/Widget/WB_Stair.WB_Stair_C|GetStoneProgressBar _wb_stair) (/ (Math|Conversions|ToFloat(Integer) _output_get_3) 2e+01))
      (Variables|Default|SetstoneFlag (== (/ (Math|Conversions|ToFloat(Integer) _output_get_3) 2e+01) 1.0))
      (elif (== ItemID 10)
        (bind _output_get_4 (Variables|Default|SetOreCurrent (Math|Integer|Min(Integer) (+ Value (stale _output_get_4)) 10)))
        (Progress|SetPercent (Variables|/Game/_BluePrint/Widget/WB_Stair.WB_Stair_C|GetOre_ProgressBar _wb_stair) (/ (Math|Conversions|ToFloat(Integer) _output_get_4) 1e+01))
        (Variables|Default|SetoreFlag (== (/ (Math|Conversions|ToFloat(Integer) _output_get_4) 1e+01) 1.0))
        (elif true
          (bind _output_get_5 (Variables|Default|SetPaldiumCurrent (Math|Integer|Min(Integer) (+ (stale _output_get_5) Value) 5)))
          (Progress|SetPercent (Variables|/Game/_BluePrint/Widget/WB_Stair.WB_Stair_C|GetPal_ProgressBar _wb_stair) (/ (Math|Conversions|ToFloat(Integer) _output_get_5) 5.0))
          (Variables|Default|SetpaldiumFlag (== (/ (Math|Conversions|ToFloat(Integer) _output_get_5) 5.0) 1.0)))))))

(event EventBeginPlay
  (bind _returnvalue (UserInterface|CreateWidget "/Game/_BluePrint/Widget/WB_Stair.WB_Stair_C"))
  (bind _output_get (Variables|Default|SetWB_Stair _returnvalue))
  (UserInterface|Viewport|AddtoViewport _output_get 0)
  (CallFunction|FlagControl false))

(event Collision|EventActorBeginOverlap
  (params (OtherActor :type Actor%20Object%20Reference)))

(event EventTick
  (params (DeltaSeconds :type Float%20%28single-precision%29))
  (if (Math|Boolean|ANDBoolean (Variables|Default|GetpaldiumFlag) (Variables|Default|GetstoneFlag) (Variables|Default|GetwoodFlag) (Variables|Default|GetoreFlag))
    (Utilities|FlowControl|DoOnce false
      (:Completed
        (CallFunction|FlagControl true)))))

(fn ConstructionScript
  (Variables|Default|SetMeshArray (Utilities|Array|MakeArray (Variables|Default|GetFloor6) (Variables|Default|GetFloor1) (Variables|Default|GetFloor2) (Variables|Default|GetFloor8) (Variables|Default|GetFloor7) (Variables|Default|GetFloor3) (Variables|Default|GetFloor4) (Variables|Default|GetFloor5) (Variables|Default|GetStair1) (Variables|Default|GetStair6) (Variables|Default|GetStair5) (Variables|Default|GetStair8) (Variables|Default|GetStair7) (Variables|Default|GetStair2) (Variables|Default|GetStair3) (Variables|Default|GetStair4))))

(fn 새함수)

(fn OnRepWoodCurrent)